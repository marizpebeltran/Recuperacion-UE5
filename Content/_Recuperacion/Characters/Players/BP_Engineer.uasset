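; BP_Engineer is the Engineer player character, which carries a battery-powered tablet with an on-screen battery display.
; On BeginPlay it caches the tablet's widget from ScreenWidget and initializes the battery bar, which RecuBattery updates thereafter.
; Tablet state changes toggle the screen and play or reverse a timeline that lerps the mesh up or down.
; RecuBattery signals become AI noise events at the actor's location, with signal strength as range.
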(event OnBatteryUpdated(RecuBattery)
  (params (CurrentBattery :type Float%20%28single-precision%29) (MaxBattery :type Float%20%28single-precision%29))
  (Default|UpdateBatteryBar (Variables|Default|GetTabletUI) CurrentBattery MaxBattery))

(event OnSignalEmitted(RecuBattery)
  (params (SignalStrength :type Float%20%28single-precision%29))
  (Class|AISenseHearing|ReportNoiseEvent (Transformation|GetActorLocation) 1.0 self SignalStrength "TabletNoise"))

(event EventBeginPlay
  (bind _aswbp_tablet_screen (Utilities|Casting|CastToWBP_TabletScreen (UserInterface|GetUserWidgetObject (Variables|Default|GetScreenWidget))))
  (bind _output_get (Variables|Default|SetTabletUI _aswbp_tablet_screen))
  (Default|UpdateBatteryBar _output_get 1e+02 1e+02))

(event Collision|EventActorBeginOverlap
  (params (OtherActor :type Actor%20Object%20Reference)))

(event EventTick
  (params (DeltaSeconds :type Float%20%28single-precision%29)))

(event EventOnTabletStateChanged
  (params (bIsActive :type Boolean))
  (if bIsActive
    (Rendering|SetVisibility (Variables|Default|GetScreenWidget) true false)
    (bind _alpha (Timeline|Anim_Tablet Play)
      (:Update
        (Transformation|SetRelativeLocation (Variables|Default|GetTabletMesh) (Math|Vector|Lerp(Vector) "50.000000,-20.000000,-50.000000" "50.000000,-20.000000,-10.000000" _alpha) false false)))
    (else
      (Rendering|SetVisibility (Variables|Default|GetScreenWidget) false false)
      (Timeline|Anim_Tablet Reverse))))

(fn ConstructionScript)